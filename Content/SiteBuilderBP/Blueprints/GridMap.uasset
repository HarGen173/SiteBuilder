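; GridMap is a tile grid layer actor that registers itself in the game state's GridMaps at its Layer index on BeginPlay.
; It fills a per-cell array with the Snow sprite's normalized tile position encoded as color and passes it to a TileArrayRT canvas render target.
; That render target feeds an M_Box dynamic material on the static mesh, so tile data reaches the shader as a texture.
; SetTiles is an unfinished stub.
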(event `self.ReceiveBeginPlay`
  (bind _assite_builder_game_state_base (cast `/Game/SiteBuilderBP/Blueprints/SiteBuilderGameStateBase` (`GameplayStatics.GetGameState`)))
  (`KismetArrayLibrary.Array_Set` (`/Game/SiteBuilderBP/Blueprints/SiteBuilderGameStateBase.GridMaps` _assite_builder_game_state_base) (`self.Layer`) self)
  (`self.CreateSpriteArray`))

(fn `CreateSpriteArray`
  (bind _spritearray (`self.SpriteArray`))
  (bind _sprite (`self.Sprite`))
  (bind _returnvalue (* (`self.SizeX`) (`self.SizeY`)))
  (bind _returnvalue_2 (- _returnvalue 1))
  (bind _returnvalue_3 (`|GenericCreateObject` "/Game/SiteBuilderBP/Blueprints/Sprite_Snow.Sprite_Snow_C" self))
  (set `self.Sprite` _returnvalue_3)
  (`KismetArrayLibrary.Array_Resize` _spritearray _returnvalue)
  (for _index (range (+ _returnvalue_2 1))
    (`KismetArrayLibrary.Array_Set` _spritearray _index (make `LinearColor` (/ (`/Game/SiteBuilderBP/Blueprints/SpriteObject.TilePositionX` _sprite) 4096.0) (/ (`/Game/SiteBuilderBP/Blueprints/SpriteObject.TilePositionY` _sprite) 2048.0))))
  (bind _returnvalue_4 (`CanvasRenderTarget2D.CreateCanvasRenderTarget2D` "/Game/SiteBuilderBP/Blueprints/TileArrayRT.TileArrayRT_C" 180 150))
  (bind _output_get (set `self.SpriteArrayRT` _returnvalue_4))
  (bind _astile_array_rt (cast `/Game/SiteBuilderBP/Blueprints/TileArrayRT` _output_get))
  (`KismetArrayLibrary.Array_Resize` (`/Game/SiteBuilderBP/Blueprints/TileArrayRT.SpriteArray` _astile_array_rt) _returnvalue_2)
  (set `/Game/SiteBuilderBP/Blueprints/TileArrayRT.SpriteArray` _spritearray _astile_array_rt)
  (bind _returnvalue_5 (`KismetMaterialLibrary.CreateDynamicMaterialInstance` "/Game/Geometry/Meshes/M_Box.M_Box"))
  (`MaterialInstanceDynamic.SetTextureParameterValue` _returnvalue_5 "TileArrayRT" _returnvalue_4)
  (`CanvasRenderTarget2D.UpdateResource` _returnvalue_4)
  (`PrimitiveComponent.SetMaterial` (`self.StaticMesh`) 0 _returnvalue_5))

(fn `SetTiles`
  (params (SizeX :type Integer) (SizeY :type Integer) (Sprite :type "PaperSprite Object Reference") (TilePositionX :type Integer) (TilePositionY :type Integer) (SpritePosition :type "Vector Structure")))

(fn `UserConstructionScript`)